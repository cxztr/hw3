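; Weapon pickup actor that gives a gun to a 0_base actor entering its Box trigger.
; On the first such overlap it plays a pickup sound at its location and calls ROSGetGun on that actor, then destroys itself.
; The call hands over the pickup's own variables for armor, damage, fire time, recoil, mesh and fire sound.
; A DoOnce after the cast limits the pickup to a single grant.
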(event OnComponentBeginOverlap(Box)
  (params (OverlappedComponent :type Primitive%20Component%20Object%20Reference) (OtherActor :type Actor%20Object%20Reference) (OtherComp :type Primitive%20Component%20Object%20Reference) (OtherBodyIndex :type Integer) (bFromSweep :type Boolean) (SweepResult :type Hit%20Result%20Structure%20%28by%20ref%29))
  (bind _as0_base (Utilities|Casting|CastTo0_base OtherActor))
  (Utilities|FlowControl|DoOnce false
    (:Completed
      (Audio|PlaySoundatLocation "/Game/weapon/WAV_getGun_Cue.WAV_getGun_Cue" (Transformation|GetActorLocation) "0, 0, 0" 1.0 1.0 0.0 0 0 0)
      (Default|ROSGetGun _as0_base (Variables|Default|Getarmor) (Variables|Default|GetgunDamage) (Variables|Default|GetgunFireTime) (Variables|Default|Getrecoil) (Variables|Default|GetnewGunMesh) (Variables|Default|GetgunFireSound))
      (Actor|DestroyActor))))

(event EventBeginPlay)

(event Collision|EventActorBeginOverlap
  (params (OtherActor :type Actor%20Object%20Reference)))

(event EventTick
  (params (DeltaSeconds :type Float%20%28single-precision%29)))

(fn ConstructionScript)